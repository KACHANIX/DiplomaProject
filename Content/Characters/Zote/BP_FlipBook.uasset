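; BP_FlipBook is an actor that displays a configurable Paper2D flipbook, keeping its material matched to the sprite currently shown.
; The construction script applies SourceFlipbook, and SetFlipbook swaps it later.
; AjustMaterial runs at construction and every Tick, copying the default material of the sprite at the playback position onto material slot 0.
; This lets each frame render with its own sprite's material.
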(event `self.ReceiveTick`
  (params (DeltaSeconds :type "Float (single-precision)"))
  (`self.AjustMaterial`))

(fn `AjustMaterial`
  (bind _paperflipbook (`self.PaperFlipbook`))
  (bind _returnvalue (`PaperFlipbook.GetSpriteAtTime` (`PaperFlipbookComponent.GetFlipbook` _paperflipbook) (`PaperFlipbookComponent.GetPlaybackPosition` _paperflipbook) false))
  (`/Engine/EditorBlueprintResources/StandardMacros.IsValid` _returnvalue
    (:`Is Valid`
      (`PrimitiveComponent.SetMaterial` _paperflipbook 0 (`PaperSprite.DefaultMaterial` _returnvalue)))))

(fn `SetFlipbook`
  (params (NewFlipbook :type "PaperFlipbook Object Reference"))
  (bind _output_get (set `self.SourceFlipbook` NewFlipbook))
  (`PaperFlipbookComponent.SetFlipbook` (`self.PaperFlipbook`) _output_get))

(fn `UserConstructionScript`
  (`PaperFlipbookComponent.SetFlipbook` (`self.PaperFlipbook`) (`self.SourceFlipbook`))
  (`self.AjustMaterial`))