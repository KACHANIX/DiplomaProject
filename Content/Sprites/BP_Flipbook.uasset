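; Flipbook actor that displays a configurable Paper2D flipbook and keeps its material matched to the sprite currently showing.
; Construction assigns SourceFlipbook to the PaperFlipbook component and applies the initial material.
; Every Tick, AdjustMaterial looks up the sprite at the current playback position and sets that sprite's default material on slot 0, allowing a different material per frame.
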(event `self.ReceiveTick`
  (params (DeltaSeconds :type "Float (single-precision)"))
  (`self.AdjustMaterial`))

(fn `AdjustMaterial`
  (bind _paperflipbook (`self.PaperFlipbook`))
  (`/Engine/EditorBlueprintResources/StandardMacros.IsValid` _paperflipbook
    (:`Is Valid`
      (`PrimitiveComponent.SetMaterial` _paperflipbook 0 (`PaperSprite.DefaultMaterial` (`PaperFlipbook.GetSpriteAtTime` (`PaperFlipbookComponent.GetFlipbook` _paperflipbook) (`PaperFlipbookComponent.GetPlaybackPosition` _paperflipbook) false))))))

(fn `SetFlipbookSource`
  (`PaperFlipbookComponent.SetFlipbook` (`self.PaperFlipbook`) (`self.SourceFlipbook`)))

(fn `UserConstructionScript`
  (`self.SetFlipbookSource`)
  (`self.AdjustMaterial`))